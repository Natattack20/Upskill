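; Behavior tree task that makes a Base_Enemy fire a short burst while the "Can See Player" blackboard key is true, finishing at once otherwise.
; A looping timer calls the enemy's Fire until the shot limit is passed, then finishes the task successfully without clearing the timer.
; While the task ticks, it snaps the enemy's capsule rotation to look at the player character's capsule.
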(event `self.ReceiveExecuteAI`
  (params (OwnerController :type "AIController Object Reference") (ControlledPawn :type "Pawn Object Reference"))
  (bind _asbase_enemy (cast `/Game/BluePrints/AI/Enemy_Prefab/Base_Enemy` ControlledPawn))
  (set `self.Amount Fired` 0)
  (if (`BlackboardComponent.GetValueAsBool` (`AIBlueprintHelperLibrary.GetBlackboard` _asbase_enemy) "Can See Player")
    (`KismetSystemLibrary.K2_SetTimerDelegate` (delegate `Fire`) 0.1 true)
    (else
      (`self.FinishExecute` true))))

(event `Fire`
  (bind _output_get (set `self.Amount Fired` (+ (`self.Amount Fired`) 1)))
  (if (> _output_get 5)
    (`self.FinishExecute` true)
    (else
      (`/Game/BluePrints/AI/Enemy_Prefab/Base_Enemy.Fire` (stale `self.ReceiveExecuteAI` _asbase_enemy)))))

(event `self.ReceiveTickAI`
  (params (OwnerController :type "AIController Object Reference") (ControlledPawn :type "Pawn Object Reference") (DeltaSeconds :type "Float (single-precision)"))
  (`SceneComponent.K2_SetWorldRotation` (`Character.CapsuleComponent` (stale `self.ReceiveExecuteAI` _asbase_enemy)) (`KismetMathLibrary.FindLookAtRotation` (`SceneComponent.K2_GetComponentLocation` (`Character.CapsuleComponent` (stale `self.ReceiveExecuteAI` _asbase_enemy))) (`SceneComponent.K2_GetComponentLocation` (`Character.CapsuleComponent` (`GameplayStatics.GetPlayerCharacter` 0)))) false false))