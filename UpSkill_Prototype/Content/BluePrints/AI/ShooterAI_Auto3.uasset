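; AI controller for a shooter enemy that runs ShooterBehaviourTree on possession and feeds it blackboard state.
; Each tick it writes the player to EnemyActor, clearing the key when the player is dead, and copies the pawn's StopShooting flag into Fire.
; Perception updates for the player set Can See Player; losing the stimulus stores LastSeen, raises Investigate and draws a debug sphere there.
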(event `self.ReceiveTick`
  (params (DeltaSeconds :type "Float (single-precision)"))
  (bind _returnvalue (`GameplayStatics.GetPlayerCharacter` 0))
  (`|ExecutionSequence`
    (:`then_0`
      (if (`/Game/BluePrints/FirstPersonBP/Blueprints/FirstPersonCharacter_Auto9.Dead` (cast `/Game/BluePrints/FirstPersonBP/Blueprints/FirstPersonCharacter_Auto9` (`GameplayStatics.GetPlayerCharacter` 0) :!pure true))
        (`BlackboardComponent.SetValueAsObject` (`self.Blackboard`) "EnemyActor" null)
        (else
          (set `self.EnemyActor` _returnvalue)
          (`BlackboardComponent.SetValueAsObject` (`self.Blackboard`) "EnemyActor" _returnvalue))))
    (:`then_1`
      (`BlackboardComponent.SetValueAsBool` (`self.Blackboard`) "Fire" (`/Game/BluePrints/AI/Enemy_Prefab/Base_Enemy.Stop Shooting` (`self.As Base Enemy`))))))

(event `self.ReceivePossess`
  (params (PossessedPawn :type "Pawn Object Reference"))
  (`self.RunBehaviorTree` "/Game/BluePrints/AI/ShooterBehaviourTree_Auto3.ShooterBehaviourTree")
  (bind _asbase_enemy (cast `/Game/BluePrints/AI/Enemy_Prefab/Base_Enemy` PossessedPawn))
  (set `self.As Base Enemy` _asbase_enemy))

(event `self.AIPerception.OnPerceptionUpdated`
  (params (UpdatedActors :type "Array of Actor Object Reference (by ref)"))
  (bind _blackboard (`self.Blackboard`))
  (bind _returnvalue (`self.K2_GetActorLocation` (`self.EnemyActor`)))
  (for _array_element UpdatedActors
    (if (== _array_element (`self.EnemyActor`))
      (bind _info (`AIPerceptionComponent.GetActorsPerception` (`self.AIPerception`) _array_element))
      (`BlackboardComponent.SetValueAsBool` _blackboard "Investigate" false)
      (bind (_age _expirationage _strength _stimuluslocation _receiverlocation _tag _bsuccessfullysensed) (break `AIStimulus` (`|GetArrayItem` (`.LastSensedStimuli` (break `ActorPerceptionBlueprintInfo` _info)))))
      (`BlackboardComponent.SetValueAsBool` _blackboard "Can See Player" _bsuccessfullysensed)
      (if (not _bsuccessfullysensed)
        (`BlackboardComponent.SetValueAsVector` _blackboard "LastSeen" _returnvalue)
        (`BlackboardComponent.SetValueAsBool` _blackboard "Investigate" true)
        (`KismetSystemLibrary.DrawDebugSphere` _returnvalue)))))

(fn `UserConstructionScript`)