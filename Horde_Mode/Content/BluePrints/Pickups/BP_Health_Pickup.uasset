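; A health pickup that heals the first-person player character on contact.
; When the box overlaps a FirstPersonCharacter whose Health is not at MaxHealth, it adds HealthGiven, caps the result at MaxHealth and destroys itself.
; A character at full health leaves the pickup in place.
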(event `self.Box.OnComponentBeginOverlap`
  (params (OverlappedComponent :type "PrimitiveComponent Object Reference") (OtherActor :type "Actor Object Reference") (OtherComp :type "PrimitiveComponent Object Reference") (OtherBodyIndex :type Integer) (bFromSweep :type Boolean) (SweepResult :type "HitResult Structure (by ref)"))
  (bind _asfirst_person_character (cast `/Game/BluePrints/FirstPersonBP/Blueprints/FirstPersonCharacter` OtherActor))
  (bind _health (`/Game/BluePrints/FirstPersonBP/Blueprints/FirstPersonCharacter.Health` _asfirst_person_character))
  (bind _max_health (`/Game/BluePrints/FirstPersonBP/Blueprints/FirstPersonCharacter.Max Health` _asfirst_person_character))
  (if (not (== _health _max_health))
    (bind _output_get (set `/Game/BluePrints/FirstPersonBP/Blueprints/FirstPersonCharacter.Health` (+ _health (`self.Health Given`)) _asfirst_person_character))
    (if (> _output_get _max_health)
      (set `/Game/BluePrints/FirstPersonBP/Blueprints/FirstPersonCharacter.Health` (`/Game/BluePrints/FirstPersonBP/Blueprints/FirstPersonCharacter.Max Health` _asfirst_person_character) _asfirst_person_character)
      (`self.K2_DestroyActor`)
      (else
        (`self.K2_DestroyActor`)))))

(fn `UserConstructionScript`)